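; BP_MyCharacter is a player character with health, alive state, coins, a toggleable flashlight and three movement speeds, driven by hard-wired key events with on-screen debug prints.
; Debug keys damage, kill or revive the player and show state, while PickCoin increments the coin count.
; Ctrl and Shift set a walking-class enum and walk speed, restoring the default on release.
; V plays a voice sound and makes noise for AI hearing.
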(event `Key|H`
  (params (Key :type "Key Structure"))
  ;[0.5573 1 0.6537] Visualización de Estado "JugadorVivo"
  (:`Pressed`
    (if (`self.IsAlive`)
      (`KismetSystemLibrary.PrintString` "Jugador vivo" true true (struct :`G` 1.0 :`B` 0.332829 :`A` 1.0))
      (else
        (`KismetSystemLibrary.PrintString` "Jugador Muerto" true true (struct :`R` 1.0 :`G` 0.072389 :`B` 0.062442 :`A` 1.0))))))

(event `Key|K`
  (params (Key :type "Key Structure"))
  ;[0.5573 1 0.6537] Cambiar el Estado del jugador "Vivo - Muerto"
  (:`Pressed`
    (if (`self.IsAlive`)
      (set `self.IsAlive` false)
      (else
        (set `self.IsAlive` true)
        (set `self.Health` 100)))
    (`KismetSystemLibrary.PrintString` "El Estado del Jugador ha cambiado")))

(event `Key|L`
  (params (Key :type "Key Structure"))
  ;[0.5573 1 0.6537] Reducción de Salud
  (:`Pressed`
    (if (<= (`self.Health`) 0)
      ;;[1 1 1] Desactivamos Flag de VIVO
      (set `self.IsAlive` false :!label _label)
      (`KismetSystemLibrary.PrintString` "Jugador ha muerto" true true (struct :`R` 1.0 :`B` 0.019289 :`A` 1.0))
      (else
        (set `self.Health` (- (`self.Health`) (`self.DamageRecieved`)))
        (`KismetSystemLibrary.PrintString` "Se ha reducido 10 de salud" true true (struct :`R` 1.0 :`G` 0.298799 :`A` 1.0))
        (if (<= (`self.Health`) 0)
          (goto _label)
          (else
            (`KismetSystemLibrary.PrintString` (`KismetStringLibrary.Concat_StrStr` "Tu salud restante es: " (`KismetStringLibrary.Conv_IntToString` (`self.Health`))))))))))

(event `Key|C`
  (params (Key :type "Key Structure"))
  ;[1 0.9581 0.4077] Visualizar cantidad actual de monedas
  (:`Pressed`
    (`KismetSystemLibrary.PrintString` (`KismetStringLibrary.Concat_StrStr` "Actualmente tienes " (`KismetStringLibrary.Conv_IntToString` (`self.Coins`)) " monedas") true true (struct :`R` 1.0 :`G` 0.825234 :`B` 0.047516 :`A` 1.0))))

(event `Key|LeftControl`
  (params (Key :type "Key Structure"))
  ;[1 0.4225 0.4923] Ajuste de Velocidad de Perosnaje dependiendo de ENUM
  (:`Pressed`
    (set `self.WalkingClass` "NewEnumerator0")
    (set `CharacterMovementComponent.MaxWalkSpeed` 200.0 (`self.CharacterMovement`))
    (`KismetSystemLibrary.PrintString` "Velocidad ajustada a 200"))
  (:`Released`
    (set `self.WalkingClass` "NewEnumerator1" :!label _label_2)
    (set `CharacterMovementComponent.MaxWalkSpeed` 500.0 (`self.CharacterMovement`))
    (`KismetSystemLibrary.PrintString` "Velocidad ajustada a 500")))

(event `Key|LeftShift`
  (params (Key :type "Key Structure"))
  ;[1 0.4225 0.4923] Ajuste de Velocidad de Perosnaje dependiendo de ENUM
  (:`Pressed`
    (set `self.WalkingClass` "NewEnumerator2")
    (set `CharacterMovementComponent.MaxWalkSpeed` 1000.0 (`self.CharacterMovement`))
    (`KismetSystemLibrary.PrintString` "Velocidad ajustada a 1000"))
  (:`Released`
    (goto _label_2)))

(event `Key|V`
  (params (Key :type "Key Structure"))
  (bind _returnvalue (`self.K2_GetActorLocation`))
  ;[0.9841 0.4375 1] Reproduccion de Voz y emisión de Ruido (para que la IA nos escuche)
  (:`Pressed`
    ;;[1 1 1] Spawneamos el sonido en la ubicacion del personaje
    (`GameplayStatics.SpawnSoundAtLocation` "/Game/Sounds/MyCharacterVoices/SC_MyVoice.SC_MyVoice" _returnvalue (struct) 1.0 1.0 0.0 null null)
    ;;[1 1 1] Hacemos Ruido para que la IA pueda oírnos (somos el instigador)
    (`self.MakeNoise` 1.0 self _returnvalue)))

(event `Key|F`
  (params (Key :type "Key Structure"))
  ;[0.03153 0.6961 1] Apagar o Prender la Linterna segun corresponda
  (:`Pressed`
    (`SceneComponent.ToggleVisibility` (`self.Linterna`) false)))

(event `Key|I`
  (params (Key :type "Key Structure"))
  (:`Pressed`
    (`/Engine/EditorBlueprintResources/StandardMacros.FlipFlop`
      (:`B`
        (`/Engine/EditorBlueprintResources/StandardMacros.IsValid` null)))))

(fn `PickCoin`
  ;[1 1 1] Incrementamos en 10 el contador de monedas
  (set `self.Coins` (+ (`self.Coins`) 10))
  (return))

(fn `UserConstructionScript`
  (`parent.UserConstructionScript`))